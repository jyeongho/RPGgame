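; Skill_AOE is a skill actor that spawns its particle effect at the player and can apply a timed speed buff.
; OnSkillNotify spawns the emitter, and Tick keeps it on the player's location.
; If the effect's display name matches the speed-up particle, walk speed rises with ArcaneLevel.
; After a delay, speed resets to a hard-coded value rather than the previous one, and the emitter deactivates.
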(event `self.OnSkillNotify`
  (bind _playerreference (`self.PlayerReference`))
  (bind _arcanelevel (`/Game/Blueprint/MoveCharBP.ArcaneLevel` _playerreference))
  (bind _charactermovement (`Character.CharacterMovement` _playerreference))
  (bind _returnvalue (`GameplayStatics.SpawnEmitterAtLocation` (`self.ParticleEffect`) (`self.K2_GetActorLocation` (`self.PlayerReference`))))
  (if (`KismetStringLibrary.EqualEqual_StrStr` (`KismetSystemLibrary.GetDisplayName` (`self.ParticleEffect`)) "P_Buff_Char_SpeedUp_01")
    (if true
      (set `CharacterMovementComponent.MaxWalkSpeed` (+ (`CharacterMovementComponent.MaxWalkSpeed` _charactermovement) (* (`KismetMathLibrary.Conv_IntToDouble` (+ _arcanelevel 1)) 400.0)) _charactermovement)
      (`KismetSystemLibrary.PrintString` (`KismetStringLibrary.Conv_IntToString` _arcanelevel))
      (`KismetSystemLibrary.Delay` 10.0)
      (set `CharacterMovementComponent.MaxWalkSpeed` 150.0 _charactermovement)
      (`ActorComponent.Deactivate` _returnvalue))))

(event `self.ReceiveTick`
  (params (DeltaSeconds :type "Float (single-precision)"))
  (`/Engine/EditorBlueprintResources/StandardMacros.IsValid` (stale `self.OnSkillNotify` _returnvalue)
    (:`Is Valid`
      (`SceneComponent.K2_SetWorldLocation` (stale `self.OnSkillNotify` _returnvalue) (`self.K2_GetActorLocation` (`self.PlayerReference`)) false false))))

(fn `UserConstructionScript`
  (`parent.UserConstructionScript`))