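; Base skill actor that handles casting, mana cost and cooldown for one player skill with staged stats.
; A cast attempt checks cooldown, casting state and mana, then plays the montage rate-scaled to the stage's cast time with movement disabled.
; Timelines resized to stage values drive the cast bar and the hotkey's cooldown material and countdown.
; OnSkillNotify only prints the skill name.
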(event `OnCooldownExpired`
  (bind _hotkey (`self.Hotkey`))
  ;[1 1 1] OnCooldownExpired
  (set `self.OnColldown` false)
  (`/Engine/EditorBlueprintResources/StandardMacros.IsValid` _hotkey
    (:`Is Valid`
      (if (not (`/Game/UI/W_SkillHotKey.Deactivated?` _hotkey))
        (`Widget.SetIsEnabled` (`/Game/UI/W_SkillHotKey.SkillButton` _hotkey) true)
        (`Image.SetColorAndOpacity` (`/Game/UI/W_SkillHotKey.SkillIcon` _hotkey) (struct :`R` 1.0 :`G` 1.0 :`B` 1.0 :`A` 1.0)))
      (`Widget.SetVisibility` (`/Game/UI/W_SkillHotKey.CooldownText` _hotkey) "Hidden")
      (`Widget.SetVisibility` (`/Game/UI/W_SkillHotKey.CooldownImage` _hotkey) "Hidden"))))

(event `OnSpellCast`
  (bind _skillanimation (`self.SkillAnimation`))
  (bind ((`RequiredSkills_42_0B722A0F4772CB092505E4BA8D90495B` _requiredskills) (`CastingTime_24_24FE27F44C5539074DB9569CF2D5B302` _castingtime)) (break `/Game/SkillSystem/Blueprints/Structures/s_SkillStage` (`self.GetCurrentStage`)))
  (bind ((`RequiredSkills_42_0B722A0F4772CB092505E4BA8D90495B` _requiredskills_2) (`CastingTime_24_24FE27F44C5539074DB9569CF2D5B302` _castingtime_2)) (break `/Game/SkillSystem/Blueprints/Structures/s_SkillStage` (`self.GetCurrentStage`)))
  (bind _returnvalue (`TimelineComponent.GetPlaybackPosition` (`self.CastingTimeline`)))
  (bind _main_widget (`/Game/Blueprint/MoveCharBP.Main Widget` (`self.PlayerReference`)))
  (bind _main_widget_2 (`/Game/Blueprint/MoveCharBP.Main Widget` (`self.PlayerReference`)))
  ;[1 1 1] OnSpellCast
  (`/Engine/EditorBlueprintResources/StandardMacros.IsValid` _skillanimation
    (:`Is Valid`
      (`self.PlayAnimation` _skillanimation (/ (`AnimSequenceBase.SequenceLength` _skillanimation) _castingtime)
        (:`Then`
          (`TextBlock.SetText` (`/Game/UI/UI_GameHUD.CastedSpellText` _main_widget_2) (`|FormatText` "Casting{SpeellName}" (`.Name_2_815547CF4ED84292D964929958422AE6` (break `/Game/SkillSystem/Blueprints/Structures/s_SkillInfo` (`self.SkillInfo`)))))
          (`ProgressBar.SetPercent` (`/Game/UI/UI_GameHUD.CastingBar` _main_widget_2) 0.0)
          (`TextBlock.SetText` (`/Game/UI/UI_GameHUD.CastTimeText` _main_widget_2) (`|FormatText` "0.0 / {CastTime}" (`KismetTextLibrary.Conv_DoubleToText` _castingtime "HalfToEven" false false 1 324 1 1)))
          (`TimelineComponent.SetTimelineLength` (`self.CastingTimeline`) _castingtime)
          (`Widget.SetVisibility` (`/Game/UI/UI_GameHUD.CastingOverlay` _main_widget_2) "HitTestInvisible")
          (`Timeline|CastingTimeline` :!via `PlayFromStart`
            (:`Update`
              (`ProgressBar.SetPercent` (`/Game/UI/UI_GameHUD.CastingBar` _main_widget) (/ _returnvalue _castingtime_2))
              (`TextBlock.SetText` (`/Game/UI/UI_GameHUD.CastTimeText` _main_widget) (`|FormatText` "{CurrentTime} / {CastTime}" (`KismetTextLibrary.Conv_DoubleToText` _returnvalue "HalfToEven" false false 1 324 0 1) (`KismetTextLibrary.Conv_DoubleToText` _castingtime_2 "HalfToEven" false false 1 324 0 1))))
            (:`Finished`
              (`Widget.SetVisibility` (`/Game/UI/UI_GameHUD.CastingOverlay` _main_widget) "Hidden"))))
        (:`Completed`
          (`self.OnCastCompleted` :!label _label))))
    (:`Is Not Valid`
      (`KismetSystemLibrary.PrintString` (`KismetTextLibrary.Conv_TextToString` (`|FormatText` "Casting {Name}" (`.Name_2_815547CF4ED84292D964929958422AE6` (break `/Game/SkillSystem/Blueprints/Structures/s_SkillInfo` (`self.SkillInfo`))))) true true (struct :`G` 0.66 :`B` 1.0 :`A` 1.0) 0.5)
      (goto _label))))

(event `OnCastCompleted`
  (bind _hotkey (`self.Hotkey`))
  (bind _hotkey_2 (`self.Hotkey`))
  (bind _cooldowntimeline (`self.CooldownTimeline`))
  (bind ((`RequiredSkills_42_0B722A0F4772CB092505E4BA8D90495B` _requiredskills) (`Cooldown_22_F68060A845F23A3583133993EE398654` _cooldown)) (break `/Game/SkillSystem/Blueprints/Structures/s_SkillStage` (`self.GetCurrentStage`)))
  (bind _returnvalue (`TimelineComponent.GetPlaybackPosition` _cooldowntimeline))
  (bind _returnvalue_2 (`TimelineComponent.GetTimelineLength` _cooldowntimeline))
  (bind _returnvalue_3 (- _returnvalue_2 _returnvalue))
  ;[1 1 1] OnCastCompleted
  (`/Game/Blueprint/MoveCharBP.EndSpellCast` (`self.PlayerReference`) self)
  (set `self.OnColldown` true)
  (set `self.CurrentlyCasted?` false)
  (`/Engine/EditorBlueprintResources/StandardMacros.IsValid` _hotkey
    (:`Is Valid`
      (`Widget.SetIsEnabled` (`/Game/UI/W_SkillHotKey.SkillButton` _hotkey) false)
      (`Image.SetColorAndOpacity` (`/Game/UI/W_SkillHotKey.SkillIcon` _hotkey) (struct :`R` 0.33 :`G` 0.33 :`B` 0.33 :`A` 1.0))
      (`MaterialInstanceDynamic.SetScalarParameterValue` (`/Game/UI/W_SkillHotKey.CooldownMat` _hotkey) "None" 1.0)
      (`TextBlock.SetText` (`/Game/UI/W_SkillHotKey.CooldownText` _hotkey) (`KismetTextLibrary.Conv_DoubleToText` _cooldown "HalfToEven" false true 1 324 0 0))
      (`Widget.SetVisibility` (`/Game/UI/W_SkillHotKey.CooldownImage` _hotkey) "HitTestInvisible")
      (`Widget.SetVisibility` (`/Game/UI/W_SkillHotKey.CooldownText` _hotkey) "HitTestInvisible"))
    (:`Is Not Valid`
      _))
  (`TimelineComponent.SetTimelineLength` (`self.CooldownTimeline`) _cooldown)
  (`Timeline|CooldownTimeline` :!via `PlayFromStart`
    (:`Update`
      (`/Engine/EditorBlueprintResources/StandardMacros.IsValid` _hotkey_2
        (:`Is Valid`
          (`MaterialInstanceDynamic.SetScalarParameterValue` (`/Game/UI/W_SkillHotKey.CooldownMat` _hotkey_2) "Percent" (- 1.0 (/ _returnvalue _returnvalue_2)))
          (`TextBlock.SetText` (`/Game/UI/W_SkillHotKey.CooldownText` _hotkey_2) (`KismetTextLibrary.Conv_DoubleToText` _returnvalue_3 "HalfToEven" false false 1 324 0 (select `bool` (> _returnvalue_3 1.0) :`false` 1))))))
    (:`Finished`
      (`self.OnCooldownExpired`))))

(event `InitializeSpellCast`
  (bind _playerreference (`self.PlayerReference`))
  ;[1 1 1] InitializeSpellCast
  (if (>= (`KismetMathLibrary.FFloor` (`/Game/Blueprint/MoveCharBP.CurrentMagic` (`self.PlayerReference`))) (`.ManaCost_31_1660579F405A242DCD01A7A245B4CF2C` (break `/Game/SkillSystem/Blueprints/Structures/s_SkillStage` (`self.GetCurrentStage`))))
    (set `self.CurrentlyCasted?` true)
    (`/Game/Blueprint/MoveCharBP.BeginSpellCast` _playerreference self)
    (set `/Game/Blueprint/MoveCharBP.CurrentMagic` (`KismetMathLibrary.Conv_IntToDouble` (- (`KismetMathLibrary.FFloor` (`/Game/Blueprint/MoveCharBP.CurrentMagic` (`self.PlayerReference`))) (`.ManaCost_31_1660579F405A242DCD01A7A245B4CF2C` (break `/Game/SkillSystem/Blueprints/Structures/s_SkillStage` (`self.GetCurrentStage`))))) _playerreference)
    (`self.OnSpellCast`)))

(event `OnTryCastSpell`
  ;[1 1 1] OntryCastSpell
  (if (and (not (`self.OnColldown`)) (not (`self.CurrentlyCasted?`)) (not (`/Game/Blueprint/MoveCharBP.IsCasting?` (`self.PlayerReference`))))
    (`self.InitializeSpellCast`)))

(event `OnSkillNotify`
  ;[1 1 1] OnSkillNotify
  (`KismetSystemLibrary.PrintString` (`KismetTextLibrary.Conv_TextToString` (`|FormatText` "Casting {Name}" (`.Name_2_815547CF4ED84292D964929958422AE6` (break `/Game/SkillSystem/Blueprints/Structures/s_SkillInfo` (`self.SkillInfo`)))))))

(fn `GetCurrentStage`
  (returns (Out :type "/Game/SkillSystem/Blueprints/Structures/s_SkillStage Structure (by ref)"))
  (return (`|GetArrayItem` (`.Stages_18_4AC8E06D49216B44DB907ABF6911F20B` (break `/Game/SkillSystem/Blueprints/Structures/s_SkillInfo` (`self.SkillInfo`))) (`self.CurrentStageIndex`))))

(fn `NextStage`
  (returns (Out :type "/Game/SkillSystem/Blueprints/Structures/s_SkillStage Structure (by ref)"))
  (bind ((`Stages_18_4AC8E06D49216B44DB907ABF6911F20B` _stages)) (break `/Game/SkillSystem/Blueprints/Structures/s_SkillInfo` (`self.SkillInfo`)))
  (return (`|GetArrayItem` _stages (`KismetMathLibrary.Clamp` (+ (`self.CurrentStageIndex`) 1) 0 (`KismetArrayLibrary.Array_LastIndex` _stages)))))

(fn `UserConstructionScript`)