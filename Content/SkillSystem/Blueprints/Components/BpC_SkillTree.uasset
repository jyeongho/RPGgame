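; Player skill tree component that manages skill points, spell upgrades and downgrades, and toggling of the tree widget on MoveCharBP.
; Upgrades are gated by points, player level and prerequisite spells; learning a spell records its class on the character and activates its tree connections.
; Point and stage changes refresh the widget's entries, with a name-based special case syncing ArcaneSight to ArcaneLevel.
; A helper finds which hotkey slot holds a skill.
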(event `self.ReceiveBeginPlay`
  (bind _asmove_char_bp (cast `/Game/Blueprint/MoveCharBP` (`self.GetOwner`)))
  (set `self.PlayCharacter` _asmove_char_bp))

(event `SetupTree`
  (bind _output_get (set `self.TreeWidget` (`/Game/UI/UI_GameHUD.SkillTree` (`/Game/Blueprint/MoveCharBP.Main Widget` (`self.PlayCharacter`)))))
  (`/Game/UI/W_MainTree.Initialize` _output_get self)
  (set `self.TreeSetUp?` true))

(event `HandleShowCommand`
  (bind _returnvalue (`GameplayStatics.GetPlayerController` 0))
  (bind _treewidget (`self.TreeWidget`))
  (if (`self.TreeSetUp?`)
    (if (`self.TreeShown?`)
      (`Widget.SetVisibility` (`self.TreeWidget`) "Hidden")
      (set `self.TreeShown?` false)
      (else
        (`Widget.SetVisibility` _treewidget "SelfHitTestInvisible")
        (`WidgetBlueprintLibrary.SetInputMode_GameAndUIEx` _returnvalue _treewidget "DoNotLock" false)
        (set `self.TreeShown?` true)
        (set `PlayerController.bShowMouseCursor` true _returnvalue)))))

(event `DowngradeSpell`
  (params (SkillActor :type "/Game/SkillSystem/Blueprints/SkillActors/Master_Skill Object Reference") (EntryWidget :type "/Game/UI/W_SkillTreeEntry Object Reference"))
  (bind _upgradedspell (`self.UpgradedSpell`))
  (bind _entrywidget (`self.EntryWidget`))
  (set `self.UpgradedSpell` SkillActor)
  (set `self.EntryWidget` EntryWidget)
  (set `/Game/SkillSystem/Blueprints/SkillActors/Master_Skill.CurrentStageIndex` (- (`/Game/SkillSystem/Blueprints/SkillActors/Master_Skill.CurrentStageIndex` _upgradedspell) 1) _upgradedspell)
  (`/Game/UI/W_SkillTreeEntry.UpdateStageText` _entrywidget)
  (`/Game/UI/W_SkillTreeEntry.UpdateIcon` _entrywidget)
  (`self.AddSkillPoints` 1)
  (`self.UpdateAllEntries`))

(event `UpgradeSpell`
  (params (SkillActor :type "/Game/SkillSystem/Blueprints/SkillActors/Master_Skill Object Reference") (EntryWidget :type "/Game/UI/W_SkillTreeEntry Object Reference"))
  (bind _upgradedspell (`self.UpgradedSpell`))
  (bind _entrywidget (`self.EntryWidget`))
  (bind _returnvalue (`GameplayStatics.GetObjectClass` (`self.UpgradedSpell`)))
  (bind _returnvalue_2 (+ (`/Game/SkillSystem/Blueprints/SkillActors/Master_Skill.CurrentStageIndex` _upgradedspell) 1))
  (bind _output_get (set `self.UpgradedSpell` SkillActor))
  (set `self.EntryWidget` EntryWidget)
  (bind _out_ (`self.CanUpgradeSpell?` _output_get))
  (if _out_
    (set `self.SkillPoints` (- (`self.SkillPoints`) 1))
    (if (`KismetStringLibrary.EqualEqual_StrStr` (`KismetTextLibrary.Conv_TextToString` (`.Name_2_815547CF4ED84292D964929958422AE6` (break `/Game/SkillSystem/Blueprints/Structures/s_SkillInfo` (`/Game/SkillSystem/Blueprints/SkillActors/Master_Skill.SkillInfo` _upgradedspell)))) "ArcaneSight")
      (set `/Game/Blueprint/MoveCharBP.ArcaneLevel` _returnvalue_2 (`self.PlayCharacter`)))
    (bind _output_get_2 (set `/Game/SkillSystem/Blueprints/SkillActors/Master_Skill.CurrentStageIndex` _returnvalue_2 _upgradedspell))
    (if (== _output_get_2 0)
      (`BlueprintSetLibrary.Set_Add` (`/Game/Blueprint/MoveCharBP.LearntSpellClasses` (`self.PlayCharacter`)) _returnvalue)
      (`/Game/UI/W_SkillTreeEntry.OnSpellLearned` (`self.EntryWidget`))
      (`self.ActivateConnections` _returnvalue))
    (`/Game/UI/W_SkillTreeEntry.UpdateStageText` _entrywidget)
    (`/Game/UI/W_SkillTreeEntry.UpdateIcon` _entrywidget)
    (`/Game/UI/W_MainTree.UpdateSP` (`self.TreeWidget`))
    (`self.UpdateAllEntries`)))

(fn `ActivateConnections`
  (params (ForSpell :type "/Game/SkillSystem/Blueprints/SkillActors/Master_Skill Class Reference"))
  (locals (localSpell :type "/Game/SkillSystem/Blueprints/SkillActors/Master_Skill Class Reference"))
  (set `local.localSpell` ForSpell)
  (for _array_element (`/Game/UI/W_MainTree.SubTreeWidgets` (`self.TreeWidget`))
    (for _array_element_2 (`/Game/UI/W_SubTree.Connections` _array_element)
      (if (== (`/Game/UI/W_Connection.ForSpell` _array_element_2) (`local.localSpell`))
        (`/Game/UI/W_Connection.Activate` _array_element_2)))))

(fn `AddSkillPoints`
  (params (Amount :type Integer))
  (set `self.SkillPoints` (+ (`self.SkillPoints`) Amount))
  (`self.UpdateAllEntries`)
  (`/Game/UI/W_MainTree.UpdateSP` (`self.TreeWidget`)))

(fn `CanUpgradeSpell?`
  (params (Spell :type "/Game/SkillSystem/Blueprints/SkillActors/Master_Skill Object Reference"))
  (returns (`Out?` :type Boolean))
  (locals (localBool :type Boolean :default true))
  (bind (_requiredlevel _requiredskills) (break `/Game/SkillSystem/Blueprints/Structures/s_SkillStage` (`/Game/SkillSystem/Blueprints/SkillActors/Master_Skill.NextStage` Spell)))
  (if (and (> (`self.SkillPoints`) 0) (>= (`/Game/Blueprint/MoveCharBP.Player Level` (`self.PlayCharacter`)) _requiredlevel) (< (`/Game/SkillSystem/Blueprints/SkillActors/Master_Skill.CurrentStageIndex` Spell) (`KismetArrayLibrary.Array_LastIndex` (`.Stages_18_4AC8E06D49216B44DB907ABF6911F20B` (break `/Game/SkillSystem/Blueprints/Structures/s_SkillInfo` (`/Game/SkillSystem/Blueprints/SkillActors/Master_Skill.SkillInfo` Spell))))))
    (for _array_element _requiredskills
      (if (not (`self.PlayerLearntSpell?` _array_element))
        (set `local.localBool` false)
        (break)))
    (return (`local.localBool`))
    (else
      (return false))))

(fn `PlayerLearntSpell?`
  (params (Spell :type "/Game/SkillSystem/Blueprints/SkillActors/Master_Skill Class Reference"))
  (returns (`Out?` :type Boolean))
  (return (`BlueprintSetLibrary.Set_Contains` (`/Game/Blueprint/MoveCharBP.LearntSpellClasses` (`self.PlayCharacter`)) Spell)))

(fn `SkillOnHotkey?`
  (params (Skill :type "/Game/SkillSystem/Blueprints/SkillActors/Master_Skill Object Reference"))
  (returns (`Out?` :type Boolean) (Hotkey :type "/Game/UI/W_SkillHotKey Object Reference"))
  (locals (localSkill :type "/Game/SkillSystem/Blueprints/SkillActors/Master_Skill Object Reference") (localOut :type Boolean) (localHotkey :type "/Game/UI/W_SkillHotKey Object Reference"))
  (set `local.localSkill` Skill)
  (for _array_element (`/Game/UI/UI_GameHUD.AllHotkeySlots` (`/Game/Blueprint/MoveCharBP.Main Widget` (`self.PlayCharacter`)))
    (bind _assignedspell (`/Game/UI/W_SkillHotKey.AssignedSpell` _array_element))
    (`/Engine/EditorBlueprintResources/StandardMacros.IsValid` _assignedspell
      (:`Is Valid`
        (if (== _assignedspell (`local.localSkill`))
          (set `local.localOut` true)
          (set `local.localHotkey` _array_element)
          (break)))))
  (return (`local.localOut`) (`local.localHotkey`)))

(fn `UpdateAllEntries`
  (for _array_element (`/Game/UI/W_MainTree.SubTreeWidgets` (`self.TreeWidget`))
    (for _array_element_2 (`/Game/UI/W_SubTree.SkillEntries` _array_element)
      (`/Game/UI/W_SkillTreeEntry.UpdateUpgradeBox` _array_element_2))))